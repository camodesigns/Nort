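; BP_Motorbyke1 is a motorbike vehicle Blueprint that turns player input into driving commands on its VehicleMovementComponent.
; The Throttle axis drives throttle when positive and otherwise feeds the brake, zeroing throttle, while Steer and HandBrake inputs map directly to steering and handbrake.
; A Debug input uses a FlipFlop to run console commands that alternate between collision debug display and lit view.
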(event `InputAction|Debug`
  (params (Key :type "Key Structure"))
  ;[1 1 1] Physics Debugging
  (:`Pressed`
    (`/Engine/EditorBlueprintResources/StandardMacros.FlipFlop`
      (:`A`
        (`KismetSystemLibrary.ExecuteConsoleCommand` "Show Collision" null)
        (`KismetSystemLibrary.ExecuteConsoleCommand` "Viewmode Viewport" null))
      (:`B`
        (`KismetSystemLibrary.ExecuteConsoleCommand` "Viewmode Lit" null)))))

(event `InputAxis|Throttle`
  (params (AxisValue :type "Float (single-precision)"))
  (bind _vehiclemovementcomponent (`self.VehicleMovementComponent`))
  ;[1 1 1] Movement Control
  (if (> AxisValue 0.0)
    (`ChaosVehicleMovementComponent.SetThrottleInput` _vehiclemovementcomponent AxisValue)
    (`ChaosVehicleMovementComponent.SetBrakeInput` _vehiclemovementcomponent 0.0)
    (else
      (bind _result (`/Engine/EditorBlueprintResources/StandardMacros.NegateFloat` AxisValue)
        (:`  `
          (`ChaosVehicleMovementComponent.SetBrakeInput` _vehiclemovementcomponent _result)
          (`ChaosVehicleMovementComponent.SetThrottleInput` _vehiclemovementcomponent 0.0))))))

(event `InputAxis|Steer`
  (params (AxisValue :type "Float (single-precision)"))
  ;[1 1 1] Movement Control
  (`ChaosVehicleMovementComponent.SetSteeringInput` (`self.VehicleMovementComponent`) AxisValue))

(event `InputAction|HandBrake`
  (params (Key :type "Key Structure"))
  (bind _vehiclemovementcomponent (`self.VehicleMovementComponent`))
  ;[1 1 1] Movement Control
  (:`Pressed`
    (`ChaosVehicleMovementComponent.SetHandbrakeInput` _vehiclemovementcomponent true))
  (:`Released`
    (`ChaosVehicleMovementComponent.SetHandbrakeInput` _vehiclemovementcomponent false)))

(fn `UserConstructionScript`)